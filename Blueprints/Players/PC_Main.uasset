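; PC_Main is the player character, with camera-relative movement, look controls, a double jump and interaction with boxes and buttons.
; Interact, gated by a can-interact flag, casts the first overlapping actor to drag a BP_Box or press a BP_Button.
; Releasing it while in the dragging state frees the first attached box.
; A player-state enum tracks jumping and dragging, and landing resets the jump counter.
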(event EventOnLanded
  (params (Hit :type Hit%20Result%20Structure%20%28by%20ref%29))
  ;[1 1 1] Jumping
  (Variables|States|Setm_JumpCounter 0))

(event Input|ActionEvents|InputActionInput_Jump
  (params (Key :type Key%20Structure))
  ;[1 1 1] Jumping
  (:Pressed
    (if (< (Variables|States|Getm_JumpCounter) 2)
      (Variables|States|Setm_PlayerState "NewEnumerator2")
      (Math|Integer|IncrementInt (Variables|States|Getm_JumpCounter)
        (:%20%20
          (Character|Jump))))))

(event Input|ActionEvents|InputActionInput_Interact
  (params (Key :type Key%20Structure))
  (bind _overlappingactors (Collision|GetOverlappingActors 0 :!class /Script/Engine.Actor))
  (bind _self self)
  (bind _output (Utilities|Array|Get(acopy) _overlappingactors))
  ;[1 1 1] Interactions
  (:Pressed
    (if (Variables|States|Getm_CanInteract)
      (bind _asbp_box (Utilities|Casting|CastToBP_Box _output)
        (:then
          (Default|BeingDragged _asbp_box _self)
          (Variables|States|Setm_PlayerState "NewEnumerator4"))
        (:CastFailed
          (bind _asbp_button (Utilities|Casting|CastToBP_Button _output))
          (Default|BeingPressed _asbp_button)))))
  (:Released
    (if (Utilities|Enum|Equal(Enum) (Variables|States|Getm_PlayerState) "NewEnumerator4")
      (bind _asbp_box_2 (Utilities|Casting|CastToBP_Box (Utilities|Array|Get(acopy) (Actor|GetAttachedActors))))
      (Default|BeingFree _asbp_box_2 _self))))

(event Input|AxisEvents|InputAxisAxis_LookX
  (params (AxisValue :type Float%20%28single-precision%29))
  ;[1 1 1] Camera controls
  (Pawn|Input|AddControllerYawInput AxisValue))

(event Input|AxisEvents|InputAxisAxis_LookY
  (params (AxisValue :type Float%20%28single-precision%29))
  ;[1 1 1] Camera controls
  (Pawn|Input|AddControllerPitchInput AxisValue))

(event Input|AxisEvents|InputAxisAxis_MoveForward
  (params (AxisValue :type Float%20%28single-precision%29))
  ;[1 1 1] Moving controls
  (Pawn|Input|AddMovementInput (Math|Vector|GetForwardVector (Variables|Default|GetCamera)) AxisValue false))

(event Input|AxisEvents|InputAxisAxis_MoveStrafe
  (params (AxisValue :type Float%20%28single-precision%29))
  ;[1 1 1] Moving controls
  (Pawn|Input|AddMovementInput (Math|Vector|GetRightVector (Variables|Default|GetCamera)) AxisValue false))

(fn ConstructionScript
  (Variables|States|Setm_PlayerState "NewEnumerator0")
  (Variables|States|Setm_JumpCounter 0)
  (Variables|States|Setm_CanInteract false))

(fn NewFunction0
  (params (self2 :type Character%20Movement%20Component%20Object%20Reference)))